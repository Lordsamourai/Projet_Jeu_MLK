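; BP_Chair is a prototype chair that makes an interacting character play a sitting animation.
; It extends the parent's StartSit and StopSit events, first calling the parent logic in each.
; StartSit casts InteractingActor to Character, stores it as SitCharacter and plays the stand-to-sit montage on it.
; StopSit stops that montage if the stored character is still valid.
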(event `self.StartSit`
  (`parent.StartSit`)
  (bind _ascharacter (cast `Character` (`self.InteractingActor`)))
  (bind _output_get (set `self.SitCharacter` _ascharacter))
  (`Character.PlayAnimMontage` _output_get "/Game/Level_1/Character/Perso_principale/Stand_To_Sit_Montage.Stand_To_Sit_Montage" 1.0 "None"))

(event `self.StopSit`
  (`parent.StopSit`)
  (bind _sitcharacter (`self.SitCharacter`)
    (:`then`
      (`Character.StopAnimMontage` _sitcharacter "/Game/Level_1/Character/Perso_principale/Stand_To_Sit_Montage.Stand_To_Sit_Montage"))
    (:`else`)))

(fn `UserConstructionScript`
  (`parent.UserConstructionScript`))