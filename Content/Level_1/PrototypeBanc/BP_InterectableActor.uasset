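; Prototype interactable actor that lets the player toggle a sit interaction while inside its Box trigger.
; On player overlap it stores the interacting actor, shows a lazily created, cached WDG_Instruction widget and enables input; leaving hides the widget and disables input.
; E toggles between StartSit and StopSit, which currently only set the Interacting flag, with StartSit also hiding the prompt and printing a debug string.
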(event `self.Box.OnComponentBeginOverlap`
  (params (OverlappedComponent :type "PrimitiveComponent Object Reference") (OtherActor :type "Actor Object Reference") (OtherComp :type "PrimitiveComponent Object Reference") (OtherBodyIndex :type Integer) (bFromSweep :type Boolean) (SweepResult :type "HitResult Structure (by ref)"))
  (bind _yes_no (message `/Game/Level_1/PrototypeBanc/BPI_Character.IsPlayer` OtherActor))
  (if _yes_no
    (set `self.InteractingActor` OtherActor)
    (`self.InstructionWidget`
      (:`then`
        _)
      (:`else`
        (bind _returnvalue (`|CreateWidget` "/Game/Level_1/PrototypeBanc/WDG_Instruction.WDG_Instruction_C"))
        (set `self.InstructionWidget` _returnvalue)))
    (`UserWidget.AddToViewport` (`self.InstructionWidget`) 0)
    (`self.EnableInput` (`GameplayStatics.GetPlayerController` 0))))

(event `self.Box.OnComponentEndOverlap`
  (params (OverlappedComponent :type "PrimitiveComponent Object Reference") (OtherActor :type "Actor Object Reference") (OtherComp :type "PrimitiveComponent Object Reference") (OtherBodyIndex :type Integer))
  (bind _yes_no (message `/Game/Level_1/PrototypeBanc/BPI_Character.IsPlayer` OtherActor))
  (if _yes_no
    (`self.HideInstruction`)
    (`self.DisableInput` (`GameplayStatics.GetPlayerController` 0))))

(event `Key|E`
  (params (Key :type "Key Structure"))
  (:`Pressed`
    (if (`self.Interacting`)
      (`self.StopSit`)
      (else
        (`self.StartSit`)))))

(event `StartSit`
  (set `self.Interacting` true)
  (`self.HideInstruction`)
  (`KismetSystemLibrary.PrintString` "Player Interracting"))

(event `StopSit`
  (set `self.Interacting` false))

(fn `UserConstructionScript`)