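; Dialogue component for a Mouse speaker that asks for cheese, then presents a poem about segregation on a merry-go-round.
; The Dialogue override switches on DialogueTreeIndex and chains AddDialogue calls through their Pass Through state.
; Finishing the poem sets the index to 1, clears progress and closes the conversation.
; Later conversations offer, in French, to reread the poem, jumping back to the same node or closing.
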(fn `CloseConversation`
  (`parent.CloseConversation`))

(fn `Dialogue`
  (`parent.Dialogue`)
  (switch `int` (`self.DialogueTreeIndex`)
    (:`0`
      (bind (_state _optionindex) (`self.AddDialogue` "Mouse" "Hi, do you have any cheese ?" (`|MakeArray` "Oui" "Non" :!type "Text")))
      (switch `/Game/Mecanique/Dialogue/Blueprint/Enum_DialogueState` _state
        (:`NewEnumerator0`
          (switch `int` _optionindex
            (:`0`
              _)
            (:`1`
              _))
          (bind (_state_2 _optionindex_2) (`self.AddDialogue` "" "Where is the Jim Crow section \nOn this merry-go-round, \nMister, cause I want to ride? \nDown South where I come from \nWhite and colored \nCan't sit side by side. \nDown South on the train \nThere's a Jim Crow car. \nOn the bus we're put in the back – \nBut there ain't no back \nTo a merry-go-round! \nWhere's the horse \nFor a kid that's black?" (`|MakeArray` "Fin" :!type "Text") :!label _label))
          (switch `/Game/Mecanique/Dialogue/Blueprint/Enum_DialogueState` _state_2
            (:`NewEnumerator0`
              (switch `int` _optionindex_2
                (:`0`
                  _)
                (:`1`
                  _))
              (`self.SetDialogueTreeIndex` 1)
              (`self.ClearDialogueProgress`)
              (`self.CloseConversation`))))))
    (:`1`
      (bind (_state_3 _optionindex_3) (`self.AddDialogue` "" "Voulez vous relire le poeme ?" (`|MakeArray` "Oui" "Non" :!type "Text")))
      (switch `/Game/Mecanique/Dialogue/Blueprint/Enum_DialogueState` _state_3
        (:`NewEnumerator0`
          (switch `int` _optionindex_3
            (:`0`
              (goto _label))
            (:`1`
              (`self.SetDialogueTreeIndex` 1)
              (`self.ClearDialogueProgress`)
              (`self.CloseConversation`))))))))