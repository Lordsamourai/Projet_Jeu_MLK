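; Dialogue component P6 that presents an English poem in a conversation, with a French prompt to reread it.
; It overrides the parent Dialogue graph, switching on DialogueTreeIndex and chaining AddDialogue steps by state and chosen option.
; Tree 0 shows a Yes/No step before the poem; tree 1 offers a reread that reuses the same poem step.
; Finishing or declining a reread sets tree 1, clears progress and closes the conversation.
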(fn `CloseConversation`
  (`parent.CloseConversation`))

(fn `Dialogue`
  (`parent.Dialogue`)
  (switch `int` (`self.DialogueTreeIndex`)
    (:`0`
      (bind (_state _optionindex) (`self.AddDialogue` "" "" (`|MakeArray` "Yes" "No" :!type "Text")))
      (switch `/Game/Mecanique/Dialogue/Blueprint/Enum_DialogueState` _state
        (:`NewEnumerator0`
          (switch `int` _optionindex
            (:`0`
              _)
            (:`1`
              _))
          (bind (_state_2 _optionindex_2) (`self.AddDialogue` "" "To fling my arms wide \nIn some place of the sun, \nTo whirl and to dance \nTill the white day is done. \nThen rest at cool evening \nBeneath a tall tree \nWhile night comes on gently, \n    Dark like me— \nThat is my dream! \nTo fling my arms wide \nIn the face of the sun, \nDance! Whirl! Whirl! \nTill the quick day is done. \nRest at pale evening . . . \nA tall, slim tree . . . \nNight coming tenderly \n    Black like me." (`|MakeArray` "Fin" :!type "Text") :!label _label))
          (switch `/Game/Mecanique/Dialogue/Blueprint/Enum_DialogueState` _state_2
            (:`NewEnumerator0`
              (switch `int` _optionindex_2
                (:`0`
                  (`self.SetDialogueTreeIndex` 1)
                  (`self.ClearDialogueProgress`)
                  (`self.CloseConversation`))))))))
    (:`1`
      (bind (_state_3 _optionindex_3) (`self.AddDialogue` "" "Voulez vous relire le poeme ?" (`|MakeArray` "Oui" "Non" :!type "Text")))
      (switch `/Game/Mecanique/Dialogue/Blueprint/Enum_DialogueState` _state_3
        (:`NewEnumerator0`
          (switch `int` _optionindex_3
            (:`0`
              (goto _label))
            (:`1`
              (`self.SetDialogueTreeIndex` 1)
              (`self.ClearDialogueProgress`)
              (`self.CloseConversation`))))))))