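; Dialogue component for the stadium (Stade): a conversation with speaker "Mouse" where the player chooses to sing the anthem or raise a fist.
; Overrides the parent Dialogue, using DialogueTreeIndex to store the choice and pick the matching ending line.
; Each ending unlocks its own achievement, plays a fade and opens the Musee level.
; In the opening cheese question, only "No" is wired to that choice.
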(fn `CloseConversation`
  (`parent.CloseConversation`))

(fn `Dialogue`
  (`parent.Dialogue`)
  (switch `int` (`self.DialogueTreeIndex`)
    (:`0`
      (bind (_state _optionindex) (`self.AddDialogue` "Mouse" "Hi, do you have any cheese ?" (`|MakeArray` "Yes" "No" :!type "Text")))
      (switch `/Game/Mecanique/Dialogue/Blueprint/Enum_DialogueState` _state
        (:`NewEnumerator0`
          (switch `int` _optionindex
            (:`1`
              (bind (_state_2 _optionindex_2) (`self.AddDialogue` "" "Que faire ?" (`|MakeArray` "Chanter l'hymne national" "Lever le poing" :!type "Text")))
              (switch `/Game/Mecanique/Dialogue/Blueprint/Enum_DialogueState` _state_2
                (:`NewEnumerator0`
                  (switch `int` _optionindex_2
                    (:`0`
                      (bind (_state_3 _optionindex_3) (`self.AddDialogue` "" "[chanter l'hymne national]" (`|MakeArray` "Fin" :!type "Text") "/Game/Audio/Hymne.Hymne"))
                      (switch `/Game/Mecanique/Dialogue/Blueprint/Enum_DialogueState` _state_3
                        (:`NewEnumerator0`
                          (switch `int` _optionindex_3
                            (:`0`
                              (`self.SetDialogueTreeIndex` 1)
                              (`self.ClearDialogueProgress`)
                              (`self.CloseConversation`))))))
                    (:`1`
                      (`self.SetDialogueTreeIndex` 2)
                      (`self.ClearDialogueProgress`)
                      (`self.CloseConversation`))))))))))
    (:`1`
      (bind _state_4 (`self.AddDialogue` "Mouse" "Vous avez était un bon petit soldat." (`|MakeArray` "Fin" :!type "Text")))
      (switch `/Game/Mecanique/Dialogue/Blueprint/Enum_DialogueState` _state_4
        (:`NewEnumerator0`
          (`self.ClearDialogueProgress`)
          (`self.CloseConversation`)
          (`AchievementSubSystem.Unlock` (subsystem `AchievementSubSystem`) "spl")
          (bind _returnvalue (`|CreateWidget` "/Game/Fade.Fade_C"))
          (`UserWidget.AddToViewport` _returnvalue 0)
          (`/Game/Fade.FadeAnim` _returnvalue)
          (`GameplayStatics.OpenLevel` "Musee"))))
    (:`2`
      (bind _state_5 (`self.AddDialogue` "Mouse" "Bravo, vous vous êtes revolter !" (`|MakeArray` "Fin" :!type "Text")))
      (switch `/Game/Mecanique/Dialogue/Blueprint/Enum_DialogueState` _state_5
        (:`NewEnumerator0`
          (`self.ClearDialogueProgress`)
          (`self.CloseConversation`)
          (`AchievementSubSystem.Unlock` (subsystem `AchievementSubSystem`) "jcts")
          (bind _returnvalue_2 (`|CreateWidget` "/Game/Fade.Fade_C"))
          (`UserWidget.AddToViewport` _returnvalue_2 0)
          (`/Game/Fade.FadeAnim` _returnvalue_2)
          (`GameplayStatics.OpenLevel` "Musee"))))))