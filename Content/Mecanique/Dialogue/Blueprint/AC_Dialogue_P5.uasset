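; Dialogue component for P5 that presents a poem about Shaft's afro as a conversation, in successive pages.
; Overrides the parent Dialogue graph, switching on DialogueTreeIndex and chaining AddDialogue nodes by state and chosen option.
; The first visit opens with a textless Yes/No prompt, and both answers lead into the poem.
; Finishing sets the index so later visits offer a French reread prompt, which replays the poem or closes the conversation.
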(fn `CloseConversation`
  (`parent.CloseConversation`))

(fn `Dialogue`
  (`parent.Dialogue`)
  (switch `int` (`self.DialogueTreeIndex`)
    (:`0`
      (bind (_state _optionindex) (`self.AddDialogue` "" "" (`|MakeArray` "Yes" "No" :!type "Text")))
      (switch `/Game/Mecanique/Dialogue/Blueprint/Enum_DialogueState` _state
        (:`NewEnumerator0`
          (switch `int` _optionindex
            (:`0`
              _)
            (:`1`
              _))
          (bind (_state_2 _optionindex_2) (`self.AddDialogue` "" "Now that my afro's as big as Shaft's  \nI feel a little better about myself.  \nHow it warms my bullet-head in Winter, \nblack halo, frizzy hat of hair.  \nShaft knew what a crown his was,  \nan orb compared to the bush \non the woman sleeping next to him.  \n(There was always a woman  \nsleeping next to him. I keep thinking, \nIf I'd only talk to strangers. . .  \ngrow a more perfect head of hair.) " (`|MakeArray` "Suite" :!type "Text") :!label _label))
          (switch `/Game/Mecanique/Dialogue/Blueprint/Enum_DialogueState` _state_2
            (:`NewEnumerator0`
              (switch `int` _optionindex_2
                (:`0`
                  _)
                (:`1`
                  _))
              (bind (_state_3 _optionindex_3) (`self.AddDialogue` "" "His afro was a crown. \nBullet after barreling bullet,  \nfist-fights & car chases,  \nthree movies & a brief TV series, \nnever one muffled strand,  \nnever dampened by sweat— \nI sweat in even the least heroic of situations. \nI'm sure you won't believe this,  \nbut if a policeman walks behind me, I tremble: \nWhat would Shaft do? What would Shaft do? \nBits of my courage flake away like dandruff. " (`|MakeArray` "Suite" :!type "Text")))
              (switch `/Game/Mecanique/Dialogue/Blueprint/Enum_DialogueState` _state_3
                (:`NewEnumerator0`
                  (switch `int` _optionindex_3
                    (:`0`
                      (bind (_state_4 _optionindex_4) (`self.AddDialogue` "" "I'm sweating even as I tell you this,  \nI'm not cool, \nI keep the real me tucked beneath a wig, \nI'm a small American frog. \nI grow beautiful as the theatre dims." (`|MakeArray` "Fin" :!type "Text")))
                      (switch `/Game/Mecanique/Dialogue/Blueprint/Enum_DialogueState` _state_4
                        (:`NewEnumerator0`
                          (switch `int` _optionindex_4
                            (:`0`
                              (`self.SetDialogueTreeIndex` 1)
                              (`self.ClearDialogueProgress`)
                              (`self.CloseConversation`))))))))))))))
    (:`1`
      (bind (_state_5 _optionindex_5) (`self.AddDialogue` "" "Voulez vous relire le poeme ?" (`|MakeArray` "Oui" "Non" :!type "Text")))
      (switch `/Game/Mecanique/Dialogue/Blueprint/Enum_DialogueState` _state_5
        (:`NewEnumerator0`
          (switch `int` _optionindex_5
            (:`0`
              (goto _label))
            (:`1`
              (`self.SetDialogueTreeIndex` 1)
              (`self.ClearDialogueProgress`)
              (`self.CloseConversation`))))))))