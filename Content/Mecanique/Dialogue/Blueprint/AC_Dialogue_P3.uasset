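; Dialogue component that recites a long English poem to the player in successive passages, then offers a replay in later conversations.
; It overrides Dialogue and branches on DialogueTreeIndex, chaining AddDialogue calls that advance through "Suite" options to a final "Fin".
; Finishing sets the index to 1, clears progress and closes the conversation.
; At index 1, a French prompt either jumps back to the first passage or closes.
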(fn `CloseConversation`
  (`parent.CloseConversation`))

(fn `Dialogue`
  (`parent.Dialogue`)
  (switch `int` (`self.DialogueTreeIndex`)
    (:`0`
      (bind (_state _optionindex) (`self.AddDialogue` "" "" (`|MakeArray` "Yes" "No" :!type "Text")))
      (switch `/Game/Mecanique/Dialogue/Blueprint/Enum_DialogueState` _state
        (:`NewEnumerator0`
          (switch `int` _optionindex
            (:`0`
              _)
            (:`1`
              _))
          (bind (_state_2 _optionindex_2) (`self.AddDialogue` "" "One sun rose on us today, kindled over our shores, \npeeking over the Smokies, greeting the faces \nof the Great Lakes, spreading a simple truth \nacross the Great Plains, then charging across the Rockies. \nOne light, waking up rooftops, under each one, a story \ntold by our silent gestures moving behind windows." (`|MakeArray` "Suite" :!type "Text") :!label _label))
          (switch `/Game/Mecanique/Dialogue/Blueprint/Enum_DialogueState` _state_2
            (:`NewEnumerator0`
              (switch `int` _optionindex_2
                (:`0`
                  _)
                (:`1`
                  _))
              (bind (_state_3 _optionindex_3) (`self.AddDialogue` "" "My face, your face, millions of faces in morning’s mirrors, \neach one yawning to life, crescendoing into our day: \npencil-yellow school buses, the rhythm of traffic lights, \nfruit stands: apples, limes, and oranges arrayed like rainbows \nbegging our praise. Silver trucks heavy with oil or paper— \nbricks or milk, teeming over highways alongside us, \non our way to clean tables, read ledgers, or save lives— \nto teach geometry, or ring-up groceries as my mother did \nfor twenty years, so I could write this poem." (`|MakeArray` "Suite" :!type "Text")))
              (switch `/Game/Mecanique/Dialogue/Blueprint/Enum_DialogueState` _state_3
                (:`NewEnumerator0`
                  (switch `int` _optionindex_3
                    (:`0`
                      (bind (_state_4 _optionindex_4) (`self.AddDialogue` "" "All of us as vital as the one light we move through, \nthe same light on blackboards with lessons for the day: \nequations to solve, history to question, or atoms imagined, \nthe “I have a dream” we keep dreaming, \nor the impossible vocabulary of sorrow that won’t explain \nthe empty desks of twenty children marked absent \ntoday, and forever. Many prayers, but one light \nbreathing color into stained glass windows, \nlife into the faces of bronze statues, warmth \nonto the steps of our museums and park benches \nas mothers watch children slide into the day." (`|MakeArray` "Suite" :!type "Text")))
                      (switch `/Game/Mecanique/Dialogue/Blueprint/Enum_DialogueState` _state_4
                        (:`NewEnumerator0`
                          (switch `int` _optionindex_4
                            (:`0`
                              (bind (_state_5 _optionindex_5) (`self.AddDialogue` "" "One ground. Our ground, rooting us to every stalk \nof corn, every head of wheat sown by sweat \nand hands, hands gleaning coal or planting windmills \nin deserts and hilltops that keep us warm, hands \ndigging trenches, routing pipes and cables, hands \nas worn as my father’s cutting sugarcane \nso my brother and I could have books and shoes. \nThe dust of farms and deserts, cities and plains \nmingled by one wind—our breath. Breathe. Hear it \nthrough the day’s gorgeous din of honking cabs, \nbuses launching down avenues, the symphony \nof footsteps, guitars, and screeching subways, \nthe unexpected song bird on your clothes line." (`|MakeArray` "Suite" :!type "Text")))
                              (switch `/Game/Mecanique/Dialogue/Blueprint/Enum_DialogueState` _state_5
                                (:`NewEnumerator0`
                                  (switch `int` _optionindex_5
                                    (:`0`
                                      (bind (_state_6 _optionindex_6) (`self.AddDialogue` "" "Hear: squeaky playground swings, trains whistling, \nor whispers across café tables, Hear: the doors we open \nfor each other all day, saying: hello / shalom, \nbuon giorno / howdy / namaste / or buenos días \nin the language my mother taught me—in every language \nspoken into one wind carrying our lives \nwithout prejudice, as these words break from my lips. \nOne sky: since the Appalachians and Sierras claimed \ntheir majesty, and the Mississippi and Colorado worked \ntheir way to the sea. Thank the work of our hands: \nweaving steel into bridges, finishing one more report \nfor the boss on time, stitching another wound \nor uniform, the first brush stroke on a portrait, \nor the last floor on the Freedom Tower \njutting into a sky that yields to our resilience." (`|MakeArray` "Suite" :!type "Text")))
                                      (switch `/Game/Mecanique/Dialogue/Blueprint/Enum_DialogueState` _state_6
                                        (:`NewEnumerator0`
                                          (switch `int` _optionindex_6
                                            (:`0`
                                              (bind (_state_7 _optionindex_7) (`self.AddDialogue` "" "One sky, toward which we sometimes lift our eyes \ntired from work: some days guessing at the weather \nof our lives, some days giving thanks for a love \nthat loves you back, sometimes praising a mother \nwho knew how to give, or forgiving a father \nwho couldn’t give what you wanted. \nWe head home: through the gloss of rain or weight \nof snow, or the plum blush of dusk, but always—home, \nalways under one sky, our sky. And always one moon \nlike a silent drum tapping on every rooftop \nand every window, of one country—all of us— \nfacing the stars \nhope—a new constellation \nwaiting for us to map it, \nwaiting for us to name it—together" (`|MakeArray` "Fin" :!type "Text")))
                                              (switch `/Game/Mecanique/Dialogue/Blueprint/Enum_DialogueState` _state_7
                                                (:`NewEnumerator0`
                                                  (switch `int` _optionindex_7
                                                    (:`0`
                                                      (`self.SetDialogueTreeIndex` 1)
                                                      (`self.ClearDialogueProgress`)
                                                      (`self.CloseConversation`))))))))))))))))))))))))))
    (:`1`
      (bind (_state_8 _optionindex_8) (`self.AddDialogue` "" "Voulez vous relire le poeme ?" (`|MakeArray` "Oui" "Non" :!type "Text")))
      (switch `/Game/Mecanique/Dialogue/Blueprint/Enum_DialogueState` _state_8
        (:`NewEnumerator0`
          (switch `int` _optionindex_8
            (:`0`
              (goto _label))
            (:`1`
              (`self.SetDialogueTreeIndex` 1)
              (`self.ClearDialogueProgress`)
              (`self.CloseConversation`))))))))