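; Dialogue component for P2 that recites Maya Angelou's poem "Still I Rise" over several pages.
; It overrides the parent Dialogue with chained AddDialogue calls, each advancing on its Pass Through state and chosen option.
; DialogueTreeIndex selects the first reading or a French re-read prompt that jumps back into the poem.
; Finishing or declining the re-read sets the index to the re-read branch, clears progress and closes the conversation.
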(fn `CloseConversation`
  (`parent.CloseConversation`))

(fn `Dialogue`
  (`parent.Dialogue`)
  (switch `int` (`self.DialogueTreeIndex`)
    (:`0`
      (bind (_state _optionindex) (`self.AddDialogue` "" "" (`|MakeArray` "Yes" "No" :!type "Text")))
      (switch `/Game/Mecanique/Dialogue/Blueprint/Enum_DialogueState` _state
        (:`NewEnumerator0`
          (switch `int` _optionindex
            (:`0`
              _)
            (:`1`
              _))
          (bind (_state_2 _optionindex_2) (`self.AddDialogue` "" "You may write me down in history \nWith your bitter, twisted lies, \nYou may trod me in the very dirt \nBut still, like dust, I'll rise. \n \nDoes my sassiness upset you? \nWhy are you beset with gloom? \n’Cause I walk like I've got oil wells \nPumping in my living room. \n \nJust like moons and like suns, \nWith the certainty of tides, \nJust like hopes springing high, \nStill I'll rise." (`|MakeArray` "Suite" :!type "Text") :!label _label))
          (switch `/Game/Mecanique/Dialogue/Blueprint/Enum_DialogueState` _state_2
            (:`NewEnumerator0`
              (switch `int` _optionindex_2
                (:`0`
                  _)
                (:`1`
                  _))
              (bind (_state_3 _optionindex_3) (`self.AddDialogue` "" "Did you want to see me broken? \nBowed head and lowered eyes? \nShoulders falling down like teardrops, \nWeakened by my soulful cries? \n \nDoes my haughtiness offend you? \nDon't you take it awful hard \n’Cause I laugh like I've got gold mines \nDiggin’ in my own backyard. \n \nYou may shoot me with your words, \nYou may cut me with your eyes, \nYou may kill me with your hatefulness, \nBut still, like air, I’ll rise." (`|MakeArray` "Suite" :!type "Text")))
              (switch `/Game/Mecanique/Dialogue/Blueprint/Enum_DialogueState` _state_3
                (:`NewEnumerator0`
                  (switch `int` _optionindex_3
                    (:`0`
                      (bind (_state_4 _optionindex_4) (`self.AddDialogue` "" "Does my sexiness upset you? \nDoes it come as a surprise \nThat I dance like I've got diamonds \nAt the meeting of my thighs? \n \nOut of the huts of history’s shame \nI rise \nUp from a past that’s rooted in pain \nI rise \nI'm a black ocean, leaping and wide, \nWelling and swelling I bear in the tide." (`|MakeArray` "Suite" :!type "Text")))
                      (switch `/Game/Mecanique/Dialogue/Blueprint/Enum_DialogueState` _state_4
                        (:`NewEnumerator0`
                          (switch `int` _optionindex_4
                            (:`0`
                              (bind (_state_5 _optionindex_5) (`self.AddDialogue` "" "Leaving behind nights of terror and fear \nI rise \nInto a daybreak that’s wondrously clear \nI rise \nBringing the gifts that my ancestors gave, \nI am the dream and the hope of the slave. \nI rise \nI rise \nI rise." (`|MakeArray` "Fin" :!type "Text")))
                              (switch `/Game/Mecanique/Dialogue/Blueprint/Enum_DialogueState` _state_5
                                (:`NewEnumerator0`
                                  (switch `int` _optionindex_5
                                    (:`0`
                                      (`self.SetDialogueTreeIndex` 1)
                                      (`self.ClearDialogueProgress`)
                                      (`self.CloseConversation`))))))))))))))))))
    (:`1`
      (bind (_state_6 _optionindex_6) (`self.AddDialogue` "" "Voulez vous relire le poeme ?" (`|MakeArray` "Oui" "Non" :!type "Text")))
      (switch `/Game/Mecanique/Dialogue/Blueprint/Enum_DialogueState` _state_6
        (:`NewEnumerator0`
          (switch `int` _optionindex_6
            (:`0`
              (goto _label))
            (:`1`
              (`self.SetDialogueTreeIndex` 1)
              (`self.ClearDialogueProgress`)
              (`self.CloseConversation`))))))))