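; Dialogue component P4, a branching conversation that presents a two-part English poem and offers to replay it.
; Overrides the parent Dialogue function, switching on DialogueTreeIndex and chaining AddDialogue nodes through their State and OptionIndex.
; The first tree opens with a Yes/No prompt, then ends the poem by setting index 1, clearing progress and closing.
; Later visits ask in French whether to reread, jumping back into the poem or closing.
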(fn `CloseConversation`
  (`parent.CloseConversation`))

(fn `Dialogue`
  (`parent.Dialogue`)
  (switch `int` (`self.DialogueTreeIndex`)
    (:`0`
      (bind (_state _optionindex) (`self.AddDialogue` "" "" (`|MakeArray` "Yes" "No" :!type "Text")))
      (switch `/Game/Mecanique/Dialogue/Blueprint/Enum_DialogueState` _state
        (:`NewEnumerator0`
          (switch `int` _optionindex
            (:`0`
              _)
            (:`1`
              _))
          (bind (_state_2 _optionindex_2) (`self.AddDialogue` "" " \nI think a lot of y’all have just been watching Dr. King get beat \n    up and, ah \n                      vacillating opportunists straining for a note of \n    militancy     and ah \nHold your great buildings on my tiny wing      or     in my tiny \n    palm      same thing different sling \nand then they shot him   and     uh               left him on the front" (`|MakeArray` "Suite" :!type "Text") :!label _label))
          (switch `/Game/Mecanique/Dialogue/Blueprint/Enum_DialogueState` _state_2
            (:`NewEnumerator0`
              (switch `int` _optionindex_2
                (:`0`
                  (bind (_state_3 _optionindex_3) (`self.AddDialogue` "" "    lawn  of everyone’s    vulgar  delirium \nfor          having been chosen       walking home that night \n     that’ll show you like    candy     and   love \ngod     openly          reverse   order \nA bird gets along beautifully in the air, but once she is on the \n    ground that special equipment hampers her a great deal. \n \n         And               Thereby home never gets to be a jaded \n             resting place." (`|MakeArray` "Fin" :!type "Text")))
                  (switch `/Game/Mecanique/Dialogue/Blueprint/Enum_DialogueState` _state_3
                    (:`NewEnumerator0`
                      (switch `int` _optionindex_3
                        (:`0`
                          (`self.SetDialogueTreeIndex` 1)
                          (`self.ClearDialogueProgress`)
                          (`self.CloseConversation`))))))))))))
    (:`1`
      (bind (_state_4 _optionindex_4) (`self.AddDialogue` "" "Voulez vous relire le poeme ?" (`|MakeArray` "Oui" "Non" :!type "Text")))
      (switch `/Game/Mecanique/Dialogue/Blueprint/Enum_DialogueState` _state_4
        (:`NewEnumerator0`
          (switch `int` _optionindex_4
            (:`0`
              (goto _label))
            (:`1`
              (`self.SetDialogueTreeIndex` 1)
              (`self.ClearDialogueProgress`)
              (`self.CloseConversation`))))))))