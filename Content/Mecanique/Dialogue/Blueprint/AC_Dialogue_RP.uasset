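; Dialogue component for the Rosa Parks scenario, where the player chooses to give up the seat or stay put.
; The Dialogue override branches on DialogueTreeIndex, saving the choice as a new index that selects the ending on a later run.
; Each ending unlocks its own achievement, starts a fade widget and opens the Musee level.
; EventGraph holds an unused variant with swapped outcome indices and no achievements or level change.
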(fn `CloseConversation`
  (`parent.CloseConversation`))

(fn `Dialogue`
  (`parent.Dialogue`)
  (switch `int` (`self.DialogueTreeIndex`)
    (:`0`
      (bind (_state _optionindex) (`self.AddDialogue` "Mouse" "Hi, do you have any cheese ?" (`|MakeArray` "Yes" "No" :!type "Text")))
      (switch `/Game/Mecanique/Dialogue/Blueprint/Enum_DialogueState` _state
        (:`NewEnumerator0`
          (switch `int` _optionindex
            (:`1`
              (bind (_state_2 _optionindex_2) (`self.AddDialogue` "" "Bouge sale negresse !" (`|MakeArray` "Se deplacer" "Ne pas bouger " :!type "Text") "/Game/Audio/Rosa_P_1.Rosa_P_1"))
              (switch `/Game/Mecanique/Dialogue/Blueprint/Enum_DialogueState` _state_2
                (:`NewEnumerator0`
                  (switch `int` _optionindex_2
                    (:`0`
                      (`self.SetDialogueTreeIndex` 2)
                      (`self.ClearDialogueProgress`)
                      (`self.CloseConversation`))
                    (:`1`
                      (bind (_state_3 _optionindex_3) (`self.AddDialogue` "" "[je suis épuisée de cette vie]" (`|MakeArray` "Fin" :!type "Text")))
                      (switch `/Game/Mecanique/Dialogue/Blueprint/Enum_DialogueState` _state_3
                        (:`NewEnumerator0`
                          (switch `int` _optionindex_3
                            (:`0`
                              (`self.SetDialogueTreeIndex` 1)
                              (`self.ClearDialogueProgress`)
                              (`self.CloseConversation`))))))))))))))
    (:`1`
      (bind _state_4 (`self.AddDialogue` "Mouse" "Bien jouer vous avez incarner Rosa Parks !! Vous pouvez etre fiere de vous !" (`|MakeArray` "Fin" :!type "Text")))
      (switch `/Game/Mecanique/Dialogue/Blueprint/Enum_DialogueState` _state_4
        (:`NewEnumerator0`
          (`self.ClearDialogueProgress`)
          (`self.CloseConversation`)
          (`AchievementSubSystem.Unlock` (subsystem `AchievementSubSystem`) "rp")
          (bind _returnvalue (`|CreateWidget` "/Game/Fade.Fade_C"))
          (`UserWidget.AddToViewport` _returnvalue 0)
          (`/Game/Fade.FadeAnim` _returnvalue)
          (`GameplayStatics.OpenLevel` "Musee"))))
    (:`2`
      (bind _state_5 (`self.AddDialogue` "Mouse" "Vous avez respecter les lois mais à quel prix ?" (`|MakeArray` "Fin" :!type "Text")))
      (switch `/Game/Mecanique/Dialogue/Blueprint/Enum_DialogueState` _state_5
        (:`NewEnumerator0`
          (`self.ClearDialogueProgress`)
          (`self.CloseConversation`)
          (`AchievementSubSystem.Unlock` (subsystem `AchievementSubSystem`) "nonrp")
          (bind _returnvalue_2 (`|CreateWidget` "/Game/Fade.Fade_C"))
          (`UserWidget.AddToViewport` _returnvalue_2 0)
          (`/Game/Fade.FadeAnim` _returnvalue_2)
          (`GameplayStatics.OpenLevel` "Musee"))))))