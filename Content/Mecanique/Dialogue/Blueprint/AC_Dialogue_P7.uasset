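; Dialogue component for P7 that presents Langston Hughes's poem "I, Too" through a conversation, overriding a parent dialogue class.
; The Dialogue graph switches on DialogueTreeIndex, chaining AddDialogue nodes that branch on state and chosen option.
; The first tree opens with a Yes/No prompt and shows the poem in two pages, then saves index 1 and closes.
; Later conversations ask in French whether to reread it, either jumping back into the poem or closing.
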(fn `CloseConversation`
  (`parent.CloseConversation`))

(fn `Dialogue`
  (`parent.Dialogue`)
  (switch `int` (`self.DialogueTreeIndex`)
    (:`0`
      (bind (_state _optionindex) (`self.AddDialogue` "" "" (`|MakeArray` "Yes" "No" :!type "Text")))
      (switch `/Game/Mecanique/Dialogue/Blueprint/Enum_DialogueState` _state
        (:`NewEnumerator0`
          (switch `int` _optionindex
            (:`0`
              _)
            (:`1`
              _))
          (bind (_state_2 _optionindex_2) (`self.AddDialogue` "" "I, too, sing America. \n \nI am the darker brother. \nThey send me to eat in the kitchen \nWhen company comes, \nBut I laugh, \nAnd eat well, \nAnd grow strong. \n" (`|MakeArray` "Suite" :!type "Text") :!label _label))
          (switch `/Game/Mecanique/Dialogue/Blueprint/Enum_DialogueState` _state_2
            (:`NewEnumerator0`
              (switch `int` _optionindex_2
                (:`0`
                  _)
                (:`1`
                  _))
              (bind (_state_3 _optionindex_3) (`self.AddDialogue` "" "Tomorrow, \nI’ll be at the table \nWhen company comes. \nNobody’ll dare \nSay to me, \n“Eat in the kitchen,” \nThen. \n \nBesides, \nThey’ll see how beautiful I am \nAnd be ashamed— \n \nI, too, am America. \n" (`|MakeArray` "Fin" :!type "Text")))
              (switch `/Game/Mecanique/Dialogue/Blueprint/Enum_DialogueState` _state_3
                (:`NewEnumerator0`
                  (switch `int` _optionindex_3
                    (:`0`
                      (`self.SetDialogueTreeIndex` 1)
                      (`self.ClearDialogueProgress`)
                      (`self.CloseConversation`))))))))))
    (:`1`
      (bind (_state_4 _optionindex_4) (`self.AddDialogue` "" "Voulez vous relire le poeme ?" (`|MakeArray` "Oui" "Non" :!type "Text")))
      (switch `/Game/Mecanique/Dialogue/Blueprint/Enum_DialogueState` _state_4
        (:`NewEnumerator0`
          (switch `int` _optionindex_4
            (:`0`
              (goto _label))
            (:`1`
              (`self.SetDialogueTreeIndex` 1)
              (`self.ClearDialogueProgress`)
              (`self.CloseConversation`))))))))