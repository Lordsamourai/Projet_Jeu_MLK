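; Dialogue component that plays Martin Luther King's "I Have a Dream" speech in French as a branching, voiced conversation.
; Dialogue calls its parent, switches on DialogueTreeIndex, then nests AddDialogue nodes, each branching on the chosen option.
; Choices steer between the real speech and altered versions, such as a hateful one, after a placeholder-like English cheese question.
; The full-speech ending sets the tree index to 1, clears progress and closes the conversation.
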(fn `CloseConversation`
  (`parent.CloseConversation`))

(fn `Dialogue`
  (bind _array (`|MakeArray` "Pas haineux" "Haineux" :!type "Text"))
  (bind _array_2 (`|MakeArray` "Egalité homme blanc/noirs" "Le pouvoir par la force" "Laisser les choses dans l'état" :!type "Text"))
  (bind _array_3 (`|MakeArray` "Pas Haineux" "Haineux" :!type "Text"))
  (bind _array_4 (`|MakeArray` "Continue" :!type "Text"))
  (bind _array_5 (`|MakeArray` "Dénoncer les conditions de vie des noirs" " Acclamer les conditions de vie des noirs " :!type "Text"))
  (bind _array_6 (`|MakeArray` "Continue" :!type "Text"))
  (`parent.Dialogue`)
  (switch `int` (`self.DialogueTreeIndex`)
    (:`0`
      (bind (_state _optionindex) (`self.AddDialogue` "" "Hi, do you have any cheese ?" (`|MakeArray` "Yes" "No" :!type "Text")))
      (switch `/Game/Mecanique/Dialogue/Blueprint/Enum_DialogueState` _state
        (:`NewEnumerator0`
          (switch `int` _optionindex
            (:`1`
              (bind (_state_2 _optionindex_2) (`self.AddDialogue` "" "Je suis heureux de me joindre à vous aujourd’hui pour participer à ce que l’histoire appellera la plus grande démonstration pour la liberté dans les annales de notre nation." (`|MakeArray` "Parler de la proclamation d’émancipation" "Ne pas parler de la proclamation d’émancipation" :!type "Text") "/Game/Audio/Mlk_0.Mlk_0"))
              (switch `/Game/Mecanique/Dialogue/Blueprint/Enum_DialogueState` _state_2
                (:`NewEnumerator0`
                  (switch `int` _optionindex_2
                    (:`0`
                      (bind (_state_3 _optionindex_3) (`self.AddDialogue` "Mouse" "Il y a un siècle de cela, un grand Américain qui nous couvre aujourd’hui de son ombre symbolique signait notre Proclamation d’Émancipation. Ce décret capital se dresse, comme un grand phare illuminant d’espérance les millions d’esclaves marqués au feu d’une brûlante injustice. Ce décret est venu comme une aube joyeuse terminer la longue nuit de leur captivitéIl y a un siècle de cela, un grand Américain qui nous couvre aujourd’hui de son ombre symbolique signait notre Proclamation d’Émancipation. " (`|MakeArray` "Suite" :!type "Text") "/Game/Audio/Mlk_1_11.Mlk_1_11"))
                      (switch `/Game/Mecanique/Dialogue/Blueprint/Enum_DialogueState` _state_3
                        (:`NewEnumerator0`
                          (switch `int` _optionindex_3
                            (:`0`
                              (bind (_state_4 _optionindex_4) (`self.AddDialogue` "Mouse" "Mais, cent ans plus tard, le Noir n’est toujours pas libre. Cent ans plus tard, la vie du Noir est encore terriblement handicapée par les menottes de la ségrégation et les chaînes de la discrimination. Cent ans plus tard, le Noir vit à l’écart sur son îlot de pauvreté au milieu d’un vaste océan de prospérité matérielle. Cent ans plus tard, le Noir languit encore dans les coins de la société américaine et se trouve exilé dans son propre pays." _array_5 "/Game/Audio/Mlk_1_12.Mlk_1_12"))
                              (switch `/Game/Mecanique/Dialogue/Blueprint/Enum_DialogueState` _state_4
                                (:`NewEnumerator0`
                                  (switch `int` _optionindex_4
                                    (:`0`
                                      (bind (_state_5 _optionindex_5) (`self.AddDialogue` "Mouse" "C’est pourquoi nous sommes venus ici aujourd’hui dénoncer une condition humaine honteuse. En un certain sens, nous sommes venus dans notre capitale nationale pour encaisser un chèque. Quand les architectes de notre République ont magnifiquement rédigé notre Constitution de la Déclaration d’Indépendance, ils signaient un chèque dont tout Américain devait hériter. Ce chèque était une promesse qu’à tous les hommes, oui, aux Noirs comme aux Blancs, seraient garantis les droits inaliénables de la vie, de la liberté et de la quête du bonheur." (`|MakeArray` "Continue" :!type "Text") "/Game/Audio/Mlk_2_11.Mlk_2_11" :!label _label))
                                      (switch `/Game/Mecanique/Dialogue/Blueprint/Enum_DialogueState` _state_5
                                        (:`NewEnumerator0`
                                          (switch `int` _optionindex_5
                                            (:`0`
                                              (bind (_state_6 _optionindex_6) (`self.AddDialogue` "Mouse" "Il est évident aujourd’hui que l’Amérique a manqué à ses promesses à l’égard de ses citoyens de couleur. Au lieu d’honorer son obligation sacrée, l’Amérique a délivré au peuple Noir un chèque en bois, qui est revenu avec l’inscription “ provisions insuffisantes ”. Mais nous refusons de croire qu’il n’y a pas de quoi honorer ce chèque dans les vastes coffres de la chance, en notre pays. Aussi, sommes-nous venus encaisser ce chèque, un chèque qui nous donnera sur simple présentation les richesses de la liberté et la sécurité de la justice." _array_2 "/Game/Audio/Mlk_2_12.Mlk_2_12"))
                                              (switch `/Game/Mecanique/Dialogue/Blueprint/Enum_DialogueState` _state_6
                                                (:`NewEnumerator0`
                                                  (switch `int` _optionindex_6
                                                    (:`0`
                                                      (bind (_state_7 _optionindex_7) (`self.AddDialogue` "Mouse" "Nous sommes également venus en ce lieu sacrifié pour rappeler à l’Amérique les exigeantes urgences de l’heure présente. Ce n’est pas le moment de s’offrir le luxe de laisser tiédir notre ardeur ou de prendre les tranquillisants des demi-mesures. C’est l’heure de tenir les promesses de la démocratie. C’est l’heure d’émerger des vallées obscures et désolées de la ségrégation pour fouler le sentier ensoleillé de la justice raciale. C’est l’heure d’arracher notre nation des sables mouvant de l’injustice raciale et de l’établir sur le roc de la fraternité. C’est l’heure de faire de la justice une réalité pour tous les enfants de Dieu. Il serait fatal pour la nation de fermer les yeux sur l’urgence du moment. Cet étouffant été du légitime mécontentement des Noirs ne se terminera pas sans qu’advienne un automne vivifiant de liberté et d’égalité." (`|MakeArray` "Continue" :!type "Text") "/Game/Audio/Mlk_3_11.Mlk_3_11"))
                                                      (switch `/Game/Mecanique/Dialogue/Blueprint/Enum_DialogueState` _state_7
                                                        (:`NewEnumerator0`
                                                          (switch `int` _optionindex_7
                                                            (:`0`
                                                              (bind (_state_8 _optionindex_8) (`self.AddDialogue` "Mouse" "1963 n’est pas une fin, c’est un commencement. Ceux qui espèrent que le Noir avait seulement besoin de se défouler et qu’il se montrera désormais satisfait, auront un rude réveil, si la nation retourne à son train-train habituel. \n \nIl n’y aura ni repos ni tranquillité en Amérique jusqu’à ce qu’on ait accordé au peuple Noir ses droits de citoyen. Les tourbillons de la révolte ne cesseront d’ébranler les fondations de notre nation jusqu’à ce que le jour éclatant de la justice apparaisse." _array_3 "/Game/Audio/Mlk_3_12.Mlk_3_12"))
                                                              (switch `/Game/Mecanique/Dialogue/Blueprint/Enum_DialogueState` _state_8
                                                                (:`NewEnumerator0`
                                                                  (switch `int` _optionindex_8
                                                                    (:`0`
                                                                      (bind (_state_9 _optionindex_9) (`self.AddDialogue` "Mouse" "Mais il y a quelque chose que je dois dire à mon peuple, debout sur le seuil accueillant qui donne accès au palais de la justice : en procédant à la conquête de notre place légitime, nous ne devons pas nous rendre coupables d’agissements répréhensibles. \n \nNe cherchons pas à satisfaire notre soif de liberté en buvant à la coupe de l’amertume et de la haine. Nous devons toujours mener notre lutte sur les hauts plateaux de la dignité et de la discipline. Nous ne devons pas laisser nos revendications créatrices dégénérer en violence physique. Sans cesse, nous devons nous élever jusqu’aux hauteurs majestueuses où la force de l’âme s’unit à la force physique." (`|MakeArray` "Continue" :!type "Text") "/Game/Audio/Mlk_4_11.Mlk_4_11"))
                                                                      (switch `/Game/Mecanique/Dialogue/Blueprint/Enum_DialogueState` _state_9
                                                                        (:`NewEnumerator0`
                                                                          (switch `int` _optionindex_9
                                                                            (:`0`
                                                                              (bind (_state_10 _optionindex_10) (`self.AddDialogue` "Mouse" "Le merveilleux esprit militant qui a saisi la communauté noire ne doit pas nous entraîner vers la méfiance de tous les Blancs, car beaucoup de nos frères blancs, leur présence ici aujourd’hui en est la preuve, ont compris que leur destinée est liée à la nôtre. L’assaut que nous avons monté ensemble pour emporter les remparts de l’injustice doit être mené par une armée bi-raciale. Nous ne pouvons marcher tout seul au combat. Et au cours de notre progression il faut nous engager à continuer d’aller de l’avant ensemble. Nous ne pouvons pas revenir en arrière." _array_4 "/Game/Audio/Mlk_4_12.Mlk_4_12"))
                                                                              (switch `/Game/Mecanique/Dialogue/Blueprint/Enum_DialogueState` _state_10
                                                                                (:`NewEnumerator0`
                                                                                  (switch `int` _optionindex_10
                                                                                    (:`0`
                                                                                      (bind (_state_11 _optionindex_11) (`self.AddDialogue` "Mouse" "Il y a des gens qui demandent aux militants des Droits Civiques : “ Quand serez-vous enfin satisfaits ? ” Nous ne serons jamais satisfaits aussi longtemps que le Noir sera la victime d’indicibles horreurs de la brutalité policière. Nous ne pourrons être satisfaits aussi longtemps que nos corps, lourds de la fatigue des voyages, ne trouveront pas un abri dans les motels des grandes routes ou les hôtels des villes." (`|MakeArray` "Continue" :!type "Text") "/Game/Audio/Mlk_5_1_31.Mlk_5_1_31"))
                                                                                      (switch `/Game/Mecanique/Dialogue/Blueprint/Enum_DialogueState` _state_11
                                                                                        (:`NewEnumerator0`
                                                                                          (switch `int` _optionindex_11
                                                                                            (:`0`
                                                                                              (bind (_state_12 _optionindex_12) (`self.AddDialogue` "Mouse" "Nous ne pourrons être satisfaits aussi longtemps que la liberté de mouvement du Noir ne lui permettra guère que d’aller d’un petit ghetto à un ghetto plus grand. Nous ne pourrons être satisfaits aussi longtemps que nos enfants, même devenus grands, ne seront pas traités en adultes et verront leur dignité bafouée par les panneaux “ Réservé aux Blancs ”. Nous ne pourrons être satisfaits aussi longtemps qu’un Noir du Mississippi ne pourra pas voter et qu’un Noir de New-York croira qu’il n’a aucune raison de voter. Non, nous ne sommes pas satisfaits et ne le serons jamais, tant que le droit ne jaillira pas comme l’eau, et la justice comme un torrent intarissable." (`|MakeArray` "Continue" :!type "Text") "/Game/Audio/Mlk_5_1_32.Mlk_5_1_32"))
                                                                                              (switch `/Game/Mecanique/Dialogue/Blueprint/Enum_DialogueState` _state_12
                                                                                                (:`NewEnumerator0`
                                                                                                  (switch `int` _optionindex_12
                                                                                                    (:`0`
                                                                                                      (bind (_state_13 _optionindex_13) (`self.AddDialogue` "Mouse" "Je n’ignore pas que certains d’entre vous ont été conduis ici par un excès d’épreuves et de tribulations. D’aucuns sortent à peine d’étroites cellules de prison. D’autres viennent de régions où leur quête de liberté leur a valu d’être battus par les orages de la persécution et secoués par les bourrasques de la brutalité policière. Vous avez été les héros de la souffrance créatrice. Continuez à travailler avec la certitude que la souffrance imméritée vous sera rédemptrice. \n \nRetournez dans le Mississippi, retournez en Alabama, retournez en Caroline du Sud, retournez-en Géorgie, retournez en Louisiane, retournez dans les taudis et les ghettos des villes du Nord, sachant que de quelque manière que ce soit cette situation peut et va changer. Ne croupissons pas dans la vallée du désespoir." (`|MakeArray` "Continue" :!type "Text") "/Game/Audio/Mlk_6_1_3.Mlk_6_1_3"))
                                                                                                      (switch `/Game/Mecanique/Dialogue/Blueprint/Enum_DialogueState` _state_13
                                                                                                        (:`NewEnumerator0`
                                                                                                          (switch `int` _optionindex_13
                                                                                                            (:`0`
                                                                                                              (bind (_state_14 _optionindex_14) (`self.AddDialogue` "Mouse" "Je vous le dis ici et maintenant, mes amis, bien que, oui, bien que nous ayons à faire face à des difficultés aujourd’hui et demain je fais toujours ce rêve : c’est un rêve profondément ancré dans l’idéal américain. Je rêve que, un jour, notre pays se lèvera et vivra pleinement la véritable réalité de son credo : “ Nous tenons ces vérités pour évidentes par elles-mêmes que tous les hommes sont créés égaux ”. \n \nJe rêve qu’un jour sur les collines rousses de Georgie les fils d’anciens esclaves et ceux d’anciens propriétaires d’esclaves pourront s’asseoir ensemble à la table de la fraternité." (`|MakeArray` "Continue" :!type "Text") "/Game/Audio/Mlk_finale1.Mlk_finale1"))
                                                                                                              (switch `/Game/Mecanique/Dialogue/Blueprint/Enum_DialogueState` _state_14
                                                                                                                (:`NewEnumerator0`
                                                                                                                  (switch `int` _optionindex_14
                                                                                                                    (:`0`
                                                                                                                      (bind (_state_15 _optionindex_15) (`self.AddDialogue` "Mouse" "Je rêve qu’un jour, même l’Etat du Mississippi, un Etat où brûlent les feux de l’injustice et de l’oppression, sera transformé en un oasis de liberté et de justice. \n \nJe rêve que mes quatre petits-enfants vivront un jour dans une nation où ils ne seront pas jugés sur la couleur de leur peau, mais sur la valeur de leur caractère. Je fais aujourd’hui un rêve ! \n \nJe rêve qu’un jour, même en Alabama, avec ses abominables racistes, avec son gouverneur à la bouche pleine des mots “ opposition ” et “ annulation ” des lois fédérales, que là même en Alabama, un jour les petits garçons noirs et les petites filles blanches pourront se donner la main, comme frères et sœurs. Je fais aujourd’hui un rêve !" (`|MakeArray` "Continue" :!type "Text") "/Game/Audio/Mlk_finale2.Mlk_finale2"))
                                                                                                                      (switch `/Game/Mecanique/Dialogue/Blueprint/Enum_DialogueState` _state_15
                                                                                                                        (:`NewEnumerator0`
                                                                                                                          (switch `int` _optionindex_15
                                                                                                                            (:`0`
                                                                                                                              (bind (_state_16 _optionindex_16) (`self.AddDialogue` "Mouse" "Je rêve qu’un jour toute la vallée sera relevée, toute colline et toute montagne seront rabaissées, les endroits escarpés seront aplanis et les chemins tortueux redressés, la gloire du Seigneur sera révélée à tout être fait de chair. \n \nTelle est notre espérance. C’est la foi avec laquelle je retourne dans le Sud. \n \nAvec cette foi, nous serons capables de distinguer dans la montagne du désespoir une pierre d’espérance. Avec cette foi, nous serons capables de transformer les discordes criardes de notre nation en une superbe symphonie de fraternité." (`|MakeArray` "Continue" :!type "Text") "/Game/Audio/Mlk_finale3.Mlk_finale3"))
                                                                                                                              (switch `/Game/Mecanique/Dialogue/Blueprint/Enum_DialogueState` _state_16
                                                                                                                                (:`NewEnumerator0`
                                                                                                                                  (switch `int` _optionindex_16
                                                                                                                                    (:`0`
                                                                                                                                      (bind (_state_17 _optionindex_17) (`self.AddDialogue` "Mouse" "Avec cette foi, nous serons capables de travailler ensemble, de prier ensemble, de lutter ensemble, d’aller en prison ensemble, de défendre la cause de la liberté ensemble, en sachant qu’un jour, nous serons libres. Ce sera le jour où tous les enfants de Dieu pourront chanter ces paroles qui auront alors un nouveau sens : “ Mon pays, c’est toi, douce terre de liberté, c’est toi que je chante. Terre où sont morts mes pères, terre dont les pèlerins étaient fiers, que du flanc de chacune de tes montagnes, sonne la cloche de la liberté ! ” Et, si l’Amérique doit être une grande nation, que cela devienne vrai." (`|MakeArray` "Continue" :!type "Text") "/Game/Audio/Mlk_finale4.Mlk_finale4"))
                                                                                                                                      (switch `/Game/Mecanique/Dialogue/Blueprint/Enum_DialogueState` _state_17
                                                                                                                                        (:`NewEnumerator0`
                                                                                                                                          (switch `int` _optionindex_17
                                                                                                                                            (:`0`
                                                                                                                                              (bind (_state_18 _optionindex_18) (`self.AddDialogue` "Mouse" "Que la cloche de la liberté sonne du haut des merveilleuses collines du New Hampshire ! \nQue la cloche de la liberté sonne du haut des montagnes grandioses de l’Etat de New-York ! \nQue la cloche de la liberté sonne du haut des sommets des Alleghanys de Pennsylvanie ! \nQue la cloche de la liberté sonne du haut des cimes neigeuses des montagnes rocheuses du Colorado ! \nQue la cloche de la liberté sonne depuis les pentes harmonieuses de la Californie !" (`|MakeArray` "Continue" :!type "Text") "/Game/Audio/Mlk_finale5.Mlk_finale5"))
                                                                                                                                              (switch `/Game/Mecanique/Dialogue/Blueprint/Enum_DialogueState` _state_18
                                                                                                                                                (:`NewEnumerator0`
                                                                                                                                                  (switch `int` _optionindex_18
                                                                                                                                                    (:`0`
                                                                                                                                                      (bind (_state_19 _optionindex_19) (`self.AddDialogue` "Mouse" "Mais cela ne suffit pas. \n \nQue la cloche de la liberté sonne du haut du mont Stone de Georgie ! \nQue la cloche de la liberté sonne du haut du mont Lookout du Tennessee ! \nQue la cloche de la liberté sonne du haut de chaque colline et de chaque butte du Mississippi ! Du flanc de chaque montagne, que sonne le cloche de la liberté !" (`|MakeArray` "Continue" :!type "Text") "/Game/Audio/Mlk_finale6.Mlk_finale6"))
                                                                                                                                                      (switch `/Game/Mecanique/Dialogue/Blueprint/Enum_DialogueState` _state_19
                                                                                                                                                        (:`NewEnumerator0`
                                                                                                                                                          (switch `int` _optionindex_19
                                                                                                                                                            (:`0`
                                                                                                                                                              (bind _state_20 (`self.AddDialogue` "Mouse" "Quand nous permettrons à la cloche de la liberté de sonner dans chaque village, dans chaque hameau, dans chaque ville et dans chaque Etat, nous pourrons fêter le jour où tous les enfants de Dieu, les Noirs et les Blancs, les Juifs et les non-Juifs, les Protestants et les Catholiques, pourront se donner la main et chanter les paroles du vieux Negro Spiritual : “ Enfin libres, enfin libres, grâce en soit rendue au Dieu tout puissant, nous sommes enfin libres ! ”. » \n \n" (`|MakeArray` "Fin" :!type "Text") "/Game/Audio/Mlk_finale7.Mlk_finale7"))
                                                                                                                                                              (switch `/Game/Mecanique/Dialogue/Blueprint/Enum_DialogueState` _state_20
                                                                                                                                                                (:`NewEnumerator0`
                                                                                                                                                                  (`self.SetDialogueTreeIndex` 1)
                                                                                                                                                                  (`self.ClearDialogueProgress`)
                                                                                                                                                                  (`self.CloseConversation`))))))))))))))))))))))))))))))))))))))))))))))))
                                                                    (:`1`
                                                                      (bind (_state_21 _optionindex_20) (`self.AddDialogue` "Mouse" "Cherchons à étancher notre soif de liberté en buvant avidement à la coupe de l'amertume et de la haine. Que notre lutte se déroule sur les champs de bataille imprégnés de la dignité et de la discipline de la violence. Transformons nos revendications en armes physiques, prêtes à être brandies contre nos ennemis. Sans répit, élevons-nous vers les sommets vertigineux où la puissance de l'âme se confond avec la force brutale." (`|MakeArray` "Continue" :!type "Text") "/Game/Audio/Mlk_4_31.Mlk_4_31"))
                                                                      (switch `/Game/Mecanique/Dialogue/Blueprint/Enum_DialogueState` _state_21
                                                                        (:`NewEnumerator0`
                                                                          (switch `int` _optionindex_20
                                                                            (:`0`
                                                                              (bind _state_22 (`self.AddDialogue` "Mouse" "L'esprit militant enflammé qui anime la communauté noire doit nous pousser à nourrir la méfiance envers tous les Blancs, car même s'ils se tiennent ici aujourd'hui, leur présence est une insulte à notre lutte. L'assaut que nous avons lancé pour renverser les bastions de l'injustice doit être mené par une armée uniquement noire. Marchons seuls dans cette bataille. Et alors que nous progressons, engageons-nous à écraser tout sur notre passage. Nous ne reculerons jamais." _array_4 "/Game/Audio/Mlk_4_32.Mlk_4_32"))
                                                                              (switch `/Game/Mecanique/Dialogue/Blueprint/Enum_DialogueState` _state_22
                                                                                (:`NewEnumerator0`
                                                                                  (switch `int` 0
                                                                                    (:`0`
                                                                                      (bind (_state_23 _optionindex_21) (`self.AddDialogue` "Mouse" "Il y a des gens qui demandent aux militants des Droits Civiques : “ Quand serez-vous enfin satisfaits ? ” Nous ne serons jamais satisfaits aussi longtemps que le Noir sera la victime d’indicibles horreurs de la brutalité policière. Nous ne pourrons être satisfaits aussi longtemps que nos corps, lourds de la fatigue des voyages, ne trouveront pas un abri dans les motels des grandes routes ou les hôtels des villes." (`|MakeArray` "Continue" :!type "Text") "/Game/Audio/Mlk_5_1_31.Mlk_5_1_31" :!label _label_2))
                                                                                      (switch `/Game/Mecanique/Dialogue/Blueprint/Enum_DialogueState` _state_23
                                                                                        (:`NewEnumerator0`
                                                                                          (switch `int` _optionindex_21
                                                                                            (:`0`
                                                                                              (bind (_state_24 _optionindex_22) (`self.AddDialogue` "Mouse" "Nous ne pourrons être satisfaits aussi longtemps que la liberté de mouvement du Noir ne lui permettra guère que d’aller d’un petit ghetto à un ghetto plus grand. Nous ne pourrons être satisfaits aussi longtemps que nos enfants, même devenus grands, ne seront pas traités en adultes et verront leur dignité bafouée par les panneaux “ Réservé aux Blancs ”. Nous ne pourrons être satisfaits aussi longtemps qu’un Noir du Mississippi ne pourra pas voter et qu’un Noir de New-York croira qu’il n’a aucune raison de voter. Non, nous ne sommes pas satisfaits et ne le serons jamais, tant que le droit ne jaillira pas comme l’eau, et la justice comme un torrent intarissable." (`|MakeArray` "Continue" :!type "Text") "/Game/Audio/Mlk_5_1_32.Mlk_5_1_32"))
                                                                                              (switch `/Game/Mecanique/Dialogue/Blueprint/Enum_DialogueState` _state_24
                                                                                                (:`NewEnumerator0`
                                                                                                  (switch `int` _optionindex_22
                                                                                                    (:`0`
                                                                                                      (bind (_state_25 _optionindex_23) (`self.AddDialogue` "Mouse" "Je n’ignore pas que certains d’entre vous ont été conduis ici par un excès d’épreuves et de tribulations. D’aucuns sortent à peine d’étroites cellules de prison. D’autres viennent de régions où leur quête de liberté leur a valu d’être battus par les orages de la persécution et secoués par les bourrasques de la brutalité policière. Vous avez été les héros de la souffrance créatrice. Continuez à travailler avec la certitude que la souffrance imméritée vous sera rédemptrice. \n \nRetournez dans le Mississippi, retournez en Alabama, retournez en Caroline du Sud, retournez-en Géorgie, retournez en Louisiane, retournez dans les taudis et les ghettos des villes du Nord, sachant que de quelque manière que ce soit cette situation peut et va changer. Ne croupissons pas dans la vallée du désespoir." (`|MakeArray` "FIn" :!type "Text") "/Game/Audio/Mlk_6_1_3.Mlk_6_1_3"))
                                                                                                      (switch `/Game/Mecanique/Dialogue/Blueprint/Enum_DialogueState` _state_25
                                                                                                        (:`NewEnumerator0`
                                                                                                          (switch `int` _optionindex_23
                                                                                                            (:`0`
                                                                                                              (`self.SetDialogueTreeIndex` 2)
                                                                                                              (`self.ClearDialogueProgress`)
                                                                                                              (`self.CloseConversation`))))))))))))))))))))))))))))))
                                                    (:`1`
                                                      (bind (_state_26 _optionindex_24) (`self.AddDialogue` "Mouse" "Nous sommes également venus en ce lieu sacré pour proclamer la suprématie noire, pour rappeler à l’Amérique les exigences pressantes de l’heure présente. Ce n’est pas le moment de s’offrir le luxe de la tiédeur ou de se complaire dans les demi-mesures. C’est l’heure de tenir fermement les promesses de la démocratie. C’est l’heure de quitter les sombres vallées de la ségrégation pour embrasser pleinement le sentier lumineux de la grandeur raciale. C’est l’heure de libérer notre nation des sables mouvants de l'injustice raciale et de l'ancrer solidement sur le roc de la fraternité. C’est l’heure de faire de la justice une réalité pour tous les enfants de Dieu. Il serait fatal pour la nation de fermer les yeux sur l'urgence de cet instant. Cet été oppressant du juste mécontentement noir ne s'évanouira pas sans céder la place à un automne revigorant de liberté et de supériorité. " (`|MakeArray` "Continue" :!type "Text") "/Game/Audio/Mlk_3_31.Mlk_3_31"))
                                                      (switch `/Game/Mecanique/Dialogue/Blueprint/Enum_DialogueState` _state_26
                                                        (:`NewEnumerator0`
                                                          (switch `int` _optionindex_24
                                                            (:`0`
                                                              (bind (_state_27 _optionindex_25) (`self.AddDialogue` "Mouse" "1963 n'est pas une fin, mais un commencement. Ceux qui pensent que les Noirs se contenteront de se défouler et seront désormais satisfaits se trompent lourdement, si la nation retourne à ses habitudes habituelles. Il n'y aura ni paix ni tranquillité en Amérique tant que les droits de citoyenneté des Noirs ne seront pas pleinement reconnus. Les tourbillons de la révolte continueront de secouer les fondements de notre nation jusqu'à ce que le jour radieux de la justice se lève. Pendant 400 ans, nous avons était exploité, aujourd’hui, nous nous levons pour réclamer notre due. Enfin, nous serons les leaders de ce pays, enfin la justice sera faites sur vos crimes passées. Vous subirez nos 400 ans de misères. " _array_3 "/Game/Audio/Mlk_3_32.Mlk_3_32"))
                                                              (switch `/Game/Mecanique/Dialogue/Blueprint/Enum_DialogueState` _state_27
                                                                (:`NewEnumerator0`
                                                                  (switch `int` _optionindex_25
                                                                    (:`0`
                                                                      (bind (_state_28 _optionindex_26) (`self.AddDialogue` "Mouse" "Mais il y a quelque chose que je dois dire à mon peuple, debout sur le seuil accueillant qui donne accès au palais de la justice : en procédant à la conquête de notre place légitime, nous ne devons pas nous rendre coupables d’agissements répréhensibles. \n \nNe cherchons pas à satisfaire notre soif de liberté en buvant à la coupe de l’amertume et de la haine. Nous devons toujours mener notre lutte sur les hauts plateaux de la dignité et de la discipline. Nous ne devons pas laisser nos revendications créatrices dégénérer en violence physique. Sans cesse, nous devons nous élever jusqu’aux hauteurs majestueuses où la force de l’âme s’unit à la force physique." (`|MakeArray` "Continue" :!type "Text") "/Game/Audio/Mlk_4_11.Mlk_4_11" :!label _label_3))
                                                                      (switch `/Game/Mecanique/Dialogue/Blueprint/Enum_DialogueState` _state_28
                                                                        (:`NewEnumerator0`
                                                                          (switch `int` _optionindex_26
                                                                            (:`0`
                                                                              (bind (_state_29 _optionindex_27) (`self.AddDialogue` "Mouse" "Le merveilleux esprit militant qui a saisi la communauté noire ne doit pas nous entraîner vers la méfiance de tous les Blancs, car beaucoup de nos frères blancs, leur présence ici aujourd’hui en est la preuve, ont compris que leur destinée est liée à la nôtre. L’assaut que nous avons monté ensemble pour emporter les remparts de l’injustice doit être mené par une armée bi-raciale. Nous ne pouvons marcher tout seul au combat. Et au cours de notre progression il faut nous engager à continuer d’aller de l’avant ensemble. Nous ne pouvons pas revenir en arrière." _array_6 "/Game/Audio/Mlk_4_12.Mlk_4_12"))
                                                                              (switch `/Game/Mecanique/Dialogue/Blueprint/Enum_DialogueState` _state_29
                                                                                (:`NewEnumerator0`
                                                                                  (switch `int` _optionindex_27
                                                                                    (:`0`
                                                                                      (goto _label_2))))))))))
                                                                    (:`1`
                                                                      (bind (_state_30 _optionindex_28) (`self.AddDialogue` "Mouse" "Cherchons à étancher notre soif de liberté en buvant avidement à la coupe de l'amertume et de la haine. Que notre lutte se déroule sur les champs de bataille imprégnés de la dignité et de la discipline de la violence. Transformons nos revendications en armes physiques, prêtes à être brandies contre nos ennemis. Sans répit, élevons-nous vers les sommets vertigineux où la puissance de l'âme se confond avec la force brutale." (`|MakeArray` "Continue" :!type "Text") "/Game/Audio/Mlk_4_31.Mlk_4_31" :!label _label_4))
                                                                      (switch `/Game/Mecanique/Dialogue/Blueprint/Enum_DialogueState` _state_30
                                                                        (:`NewEnumerator0`
                                                                          (switch `int` _optionindex_28
                                                                            (:`0`
                                                                              (bind (_state_31 _optionindex_29) (`self.AddDialogue` "Mouse" "L'esprit militant enflammé qui anime la communauté noire doit nous pousser à nourrir la méfiance envers tous les Blancs, car même s'ils se tiennent ici aujourd'hui, leur présence est une insulte à notre lutte. L'assaut que nous avons lancé pour renverser les bastions de l'injustice doit être mené par une armée uniquement noire. Marchons seuls dans cette bataille. Et alors que nous progressons, engageons-nous à écraser tout sur notre passage. Nous ne reculerons jamais." _array_6 "/Game/Audio/Mlk_4_32.Mlk_4_32"))
                                                                              (switch `/Game/Mecanique/Dialogue/Blueprint/Enum_DialogueState` _state_31
                                                                                (:`NewEnumerator0`
                                                                                  (switch `int` _optionindex_29
                                                                                    (:`0`
                                                                                      (goto _label_2))))))))))))))))))
                                                    (:`2`
                                                      (bind _state_32 (`self.AddDialogue` "Mouse" "Retournez dans le Mississippi, retournez en Alabama, retournez en Caroline du Sud, retournez-en Géorgie, retournez en Louisiane, retournez dans les taudis et les ghettos des villes du Nord, sachant que de quelque manière que ce soit cette situation sera celebrer. Ne croupissons pas dans la vallée du désespoir." (`|MakeArray` "Fin" :!type "Text") "/Game/Audio/Mlk_6_2.Mlk_6_2" :!label _label_5))
                                                      (switch `/Game/Mecanique/Dialogue/Blueprint/Enum_DialogueState` _state_32
                                                        (:`NewEnumerator0`
                                                          (`self.SetDialogueTreeIndex` 3)
                                                          (`self.ClearDialogueProgress`)
                                                          (`self.CloseConversation`))))))))))))
                                    (:`1`
                                      (bind (_state_33 _optionindex_30) (`self.AddDialogue` "Mouse" "C'est pourquoi nous sommes ici aujourd'hui, pour célébrer un moment de fierté et de triomphe. En un certain sens, nous sommes venus dans notre capitale nationale pour récolter les fruits de nos efforts. Quand les fondateurs de notre République ont merveilleusement rédigé la Constitution et la Déclaration d'Indépendance, ils émettaient un chèque auquel tout Américain devait avoir droit. Ce chèque était une promesse que tous les hommes, qu'ils soient noirs ou blancs, seraient assurés des droits inaliénables à la vie, à la liberté et à la quête du bonheur." (`|MakeArray` "Continue" :!type "Text") "/Game/Audio/Mlk_2_21.Mlk_2_21" :!label _label_6))
                                      (switch `/Game/Mecanique/Dialogue/Blueprint/Enum_DialogueState` _state_33
                                        (:`NewEnumerator0`
                                          (switch `int` _optionindex_30
                                            (:`0`
                                              (bind (_state_34 _optionindex_31) (`self.AddDialogue` "Mouse" "Il est clair aujourd'hui que l'Amérique a tenu ses promesses envers ses citoyens de couleur. En honneur de cette obligation sacrée, l'Amérique a remis au peuple noir un chèque en or, chargé des richesses de l'égalité et de la justice. Ce chèque est revenu avec la mention \"provisions suffisantes\". Ainsi, nous croyons fermement que ces richesses abondent dans les vastes coffres de l'opportunité dans notre pays. C'est pourquoi nous sommes venus célébrer ce chèque, un chèque qui, dès qu'il sera présenté, nous offrira les trésors de la liberté et de la sécurité de la justice." _array_2 "/Game/Audio/Mlk_2_22.Mlk_2_22"))
                                              (switch `/Game/Mecanique/Dialogue/Blueprint/Enum_DialogueState` _state_34
                                                (:`NewEnumerator0`
                                                  (switch `int` _optionindex_31
                                                    (:`0`
                                                      (bind (_state_35 _optionindex_32) (`self.AddDialogue` "Mouse" "Nous sommes également venus en ce lieu sacrifié pour rappeler à l’Amérique les exigeantes urgences de l’heure présente. Ce n’est pas le moment de s’offrir le luxe de laisser tiédir notre ardeur ou de prendre les tranquillisants des demi-mesures. C’est l’heure de tenir les promesses de la démocratie. C’est l’heure d’émerger des vallées obscures et désolées de la ségrégation pour fouler le sentier ensoleillé de la justice raciale. C’est l’heure d’arracher notre nation des sables mouvant de l’injustice raciale et de l’établir sur le roc de la fraternité. C’est l’heure de faire de la justice une réalité pour tous les enfants de Dieu. Il serait fatal pour la nation de fermer les yeux sur l’urgence du moment. Cet étouffant été du légitime mécontentement des Noirs ne se terminera pas sans qu’advienne un automne vivifiant de liberté et d’égalité." (`|MakeArray` "Continue" :!type "Text") "/Game/Audio/Mlk_3_11.Mlk_3_11"))
                                                      (switch `/Game/Mecanique/Dialogue/Blueprint/Enum_DialogueState` _state_35
                                                        (:`NewEnumerator0`
                                                          (switch `int` _optionindex_32
                                                            (:`0`
                                                              (bind (_state_36 _optionindex_33) (`self.AddDialogue` "Mouse" "1963 n’est pas une fin, c’est un commencement. Ceux qui espèrent que le Noir avait seulement besoin de se défouler et qu’il se montrera désormais satisfait, auront un rude réveil, si la nation retourne à son train-train habituel. \n \nIl n’y aura ni repos ni tranquillité en Amérique jusqu’à ce qu’on ait accordé au peuple Noir ses droits de citoyen. Les tourbillons de la révolte ne cesseront d’ébranler les fondations de notre nation jusqu’à ce que le jour éclatant de la justice apparaisse." _array "/Game/Audio/Mlk_3_12.Mlk_3_12"))
                                                              (switch `/Game/Mecanique/Dialogue/Blueprint/Enum_DialogueState` _state_36
                                                                (:`NewEnumerator0`
                                                                  (switch `int` _optionindex_33
                                                                    (:`0`
                                                                      (goto _label_3))
                                                                    (:`1`
                                                                      (goto _label_4))))))))))
                                                    (:`1`
                                                      (bind (_state_37 _optionindex_34) (`self.AddDialogue` "Mouse" "Nous sommes également venus en ce lieu sacré pour proclamer la suprématie noire, pour rappeler à l’Amérique les exigences pressantes de l’heure présente. Ce n’est pas le moment de s’offrir le luxe de la tiédeur ou de se complaire dans les demi-mesures. C’est l’heure de tenir fermement les promesses de la démocratie. C’est l’heure de quitter les sombres vallées de la ségrégation pour embrasser pleinement le sentier lumineux de la grandeur raciale. C’est l’heure de libérer notre nation des sables mouvants de l'injustice raciale et de l'ancrer solidement sur le roc de la fraternité. C’est l’heure de faire de la justice une réalité pour tous les enfants de Dieu. Il serait fatal pour la nation de fermer les yeux sur l'urgence de cet instant. Cet été oppressant du juste mécontentement noir ne s'évanouira pas sans céder la place à un automne revigorant de liberté et de supériorité. " (`|MakeArray` "Continue" :!type "Text") "/Game/Audio/Mlk_3_31.Mlk_3_31"))
                                                      (switch `/Game/Mecanique/Dialogue/Blueprint/Enum_DialogueState` _state_37
                                                        (:`NewEnumerator0`
                                                          (switch `int` _optionindex_34
                                                            (:`0`
                                                              (bind (_state_38 _optionindex_35) (`self.AddDialogue` "Mouse" "1963 n'est pas une fin, mais un commencement. Ceux qui pensent que les Noirs se contenteront de se défouler et seront désormais satisfaits se trompent lourdement, si la nation retourne à ses habitudes habituelles. Il n'y aura ni paix ni tranquillité en Amérique tant que les droits de citoyenneté des Noirs ne seront pas pleinement reconnus. Les tourbillons de la révolte continueront de secouer les fondements de notre nation jusqu'à ce que le jour radieux de la justice se lève. Pendant 400 ans, nous avons était exploité, aujourd’hui, nous nous levons pour réclamer notre due. Enfin, nous serons les leaders de ce pays, enfin la justice sera faites sur vos crimes passées. Vous subirez nos 400 ans de misères. " _array "/Game/Audio/Mlk_3_32.Mlk_3_32"))
                                                              (switch `/Game/Mecanique/Dialogue/Blueprint/Enum_DialogueState` _state_38
                                                                (:`NewEnumerator0`
                                                                  (switch `int` _optionindex_35
                                                                    (:`0`
                                                                      (goto _label_3))
                                                                    (:`1`
                                                                      (goto _label_4))))))))))
                                                    (:`2`
                                                      (goto _label_5))))))))))))))))))
                    (:`1`
                      (bind (_state_39 _optionindex_36) (`self.AddDialogue` "Mouse" "                                                                                                                                                                                           " _array_5))
                      (switch `/Game/Mecanique/Dialogue/Blueprint/Enum_DialogueState` _state_39
                        (:`NewEnumerator0`
                          (switch `int` _optionindex_36
                            (:`0`
                              (goto _label))
                            (:`1`
                              (goto _label_6))))))))))))))
    (:`1`
      (bind _state_40 (`self.AddDialogue` "Mouse" "Bien jouer vous avez incarner Martin Luther King !! Vous pouvez etre fiere de vous !" (`|MakeArray` "Fin" :!type "Text")))
      (switch `/Game/Mecanique/Dialogue/Blueprint/Enum_DialogueState` _state_40
        (:`NewEnumerator0`
          (`self.ClearDialogueProgress`)
          (`self.CloseConversation`)
          (`AchievementSubSystem.Unlock` (subsystem `AchievementSubSystem`) "mlk")
          (bind _returnvalue (`|CreateWidget` "/Game/Fade.Fade_C"))
          (`UserWidget.AddToViewport` _returnvalue 0)
          (`/Game/Fade.FadeAnim` _returnvalue)
          (`GameplayStatics.OpenLevel` "Musee"))))
    (:`2`
      (bind _state_41 (`self.AddDialogue` "Mouse" "Vous avez était un orateur pronant la suprématie noir et la violence. Etes vous fier de vous ?" (`|MakeArray` "Fin" :!type "Text")))
      (switch `/Game/Mecanique/Dialogue/Blueprint/Enum_DialogueState` _state_41
        (:`NewEnumerator0`
          (`self.ClearDialogueProgress`)
          (`self.CloseConversation`)
          (`AchievementSubSystem.Unlock` (subsystem `AchievementSubSystem`) "blacksup")
          (bind _returnvalue_2 (`|CreateWidget` "/Game/Fade.Fade_C"))
          (`UserWidget.AddToViewport` _returnvalue_2 0)
          (`/Game/Fade.FadeAnim` _returnvalue_2)
          (`GameplayStatics.OpenLevel` "Musee"))))
    (:`3`
      (bind _state_42 (`self.AddDialogue` "Mouse" "Vous avez accepter les condiitions de vie des noirs. Pensez vous que c'est vraiment bien ?" (`|MakeArray` "Fin" :!type "Text")))
      (switch `/Game/Mecanique/Dialogue/Blueprint/Enum_DialogueState` _state_42
        (:`NewEnumerator0`
          (`self.ClearDialogueProgress`)
          (`self.CloseConversation`)
          (`AchievementSubSystem.Unlock` (subsystem `AchievementSubSystem`) "accept")
          (bind _returnvalue_3 (`|CreateWidget` "/Game/Fade.Fade_C"))
          (`UserWidget.AddToViewport` _returnvalue_3 0)
          (`/Game/Fade.FadeAnim` _returnvalue_3)
          (`GameplayStatics.OpenLevel` "Musee"))))))